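; BP_PawnBall is a ball actor that rolls toward a supplied target location.
; GetDestination sets direction and remaining distance, with speed scaled by that distance and capped so the ball slows near the target.
; Tick applies an unswept offset clamped to the stored distance and spins the mesh about the axis perpendicular to travel, matching roll to movement.
; The construction script raises the mesh by BallHeight, which also serves as the rolling radius.
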(event Custom|GetDestination
  (params (TargetLocation :type Vector))
  (bind _returnvalue (Transformation|GetActorLocation))
  (bind _returnvalue_2 (- TargetLocation _returnvalue))
  (bind _returnvalue_3 (Math|Vector|VectorLength _returnvalue_2))
  (Variables|Default|SetDirection (Math|Vector|Normalize _returnvalue_2))
  (Variables|Default|SetDistance _returnvalue_3)
  (Variables|Default|SetSpeed (Math|Float|MapRangeClamped _returnvalue_3 0.0 2.8e+03 0.0 1e+03)))

(event EventTick
  (params (DeltaSeconds :type Float%20%28single-precision%29))
  (bind _returnvalue (Utilities|Time|GetWorldDeltaSeconds))
  (bind _distance (Variables|Default|GetDistance))
  (bind _speed (Variables|Default|GetSpeed))
  (bind _returnvalue_2 (* _speed _returnvalue))
  (bind _returnvalue_3 (Math|Float|Min(Float) _returnvalue_2 _distance))
  (Transformation|AddActorLocalOffset (* (Variables|Default|GetDirection) _returnvalue_3) false false)
  (Transformation|AddWorldRotation (Variables|Default|GetBallMesh) (Math|Vector|RotatorfromAxisandAngle (Math|Vector|CrossProduct "0, 0,1.000000" (Variables|Default|GetDirection)) (Math|Trig|RadiansToDegrees (/ _returnvalue_3 (Variables|Default|GetBallHeight)))) false false))

(fn ConstructionScript
  (Transformation|SetRelativeLocation (Variables|Default|GetBallMesh) (Math|Vector|MakeVector 0.0 0.0 (Variables|Default|GetBallHeight)) false false))