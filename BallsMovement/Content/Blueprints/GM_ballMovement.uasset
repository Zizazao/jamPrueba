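; GM_ballMovement, by its prefix a game mode for a ball movement game, builds the ball menu UI when play begins.
; It creates a WD_ballMenu widget and adds it to the viewport.
; It then reads every row of the BallProps data table, creating a WD_HorizontalMenu entry with that row's icon and adding it to the menu's horizontal container, so the menu is data-driven.
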(event EventBeginPlay
  (bind _ballprops (Variables|Default|GetBallProps))
  (bind _returnvalue (UserInterface|CreateWidget "/Game/Widgets/WD_ballMenu.WD_ballMenu_C"))
  (bind _output_get (Variables|Default|SetWidget _returnvalue))
  (UserInterface|Viewport|AddtoViewport _output_get 0)
  (bind _outrownames (DataTable|GetDataTableRowNames _ballprops))
  (for _array_element _outrownames
    (bind _returnvalue_2 (Utilities|GetDataTableRow _ballprops _array_element)
      (:then
        (bind _returnvalue_3 (UserInterface|CreateWidget "/Game/Widgets/WD_HorizontalMenu.WD_HorizontalMenu_C"))
        (Appearance|SetBrushfromTexture (Variables|/Game/Widgets/WD_HorizontalMenu.WD_HorizontalMenu_C|GetImage_0 _returnvalue_3) (Utilities|Struct|BreakS_BallProps _returnvalue_2) false)
        (Widget|Panel|AddChild (Variables|/Game/Widgets/WD_ballMenu.WD_ballMenu_C|GetHorizontalMenu (Variables|Default|GetWidget)) _returnvalue_3)))))

(fn ConstructionScript)